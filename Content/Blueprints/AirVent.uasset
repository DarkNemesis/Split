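; Air vent actor that pushes a character along its arrow's forward direction while inside the trigger.
; BeginPlay sizes the trigger using the actor's X and Y scale and a configurable Z size.
; Overlap events store or clear a single tracked actor, regardless of which actor leaves.
; Tick applies a mass-dependent impulse to that actor's CharacterMovementComponent every frame, without delta-time scaling.
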(event `self.ReceiveBeginPlay`
  (`SceneComponent.SetWorldScale3D` (`self.mAirTrigger`) (`KismetMathLibrary.MakeVector` (.x (`self.GetActorScale3D`)) (.y (`self.GetActorScale3D`)) (`self.mSize`))))

(event `self.ReceiveTick`
  (params (DeltaSeconds :type "Float (single-precision)"))
  (bind _mactor (`self.mActor`))
  (`/Engine/EditorBlueprintResources/StandardMacros.IsValid` _mactor
    (:`Is Valid`
      (`CharacterMovementComponent.AddImpulse` (`self.GetComponentByClass` _mactor "/Script/Engine.CharacterMovementComponent") (* (`SceneComponent.GetForwardVector` (`self.Arrow`)) (`self.mForce`)) false))))

(event `self.mAirTrigger.OnComponentBeginOverlap`
  (params (OverlappedComponent :type "PrimitiveComponent Object Reference") (OtherActor :type "Actor Object Reference") (OtherComp :type "PrimitiveComponent Object Reference") (OtherBodyIndex :type Integer) (bFromSweep :type Boolean) (SweepResult :type "HitResult Structure (by ref)"))
  ;[1 1 1] Comment
  (set `self.mActor` OtherActor))

(event `self.mAirTrigger.OnComponentEndOverlap`
  (params (OverlappedComponent :type "PrimitiveComponent Object Reference") (OtherActor :type "Actor Object Reference") (OtherComp :type "PrimitiveComponent Object Reference") (OtherBodyIndex :type Integer))
  ;[1 1 1] Comment
  (set `self.mActor` null))

(fn `UserConstructionScript`)