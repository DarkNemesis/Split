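; Controller for a character split into skeleton, skin and muscle pawns, handling switching, walking and bone throwing.
; Switch cycles player possession through the three, swapping the walk sound; Throw, only as skeleton, spawns a Bone targeted sideways along Y by facing.
; Tick polls A/D to play that sound and set a Y force, applied every frame to the possessed pawn and never zeroed on release.
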(event `self.ReceiveBeginPlay`
  (set `self.mCurrentSound` (`self.mSkeletonSound`)))

(event `InputAction|Throw`
  (params (Key :type "Key Structure"))
  (bind (_returnvalue_x _returnvalue_y) (`KismetMathLibrary.BreakVector` (`self.GetActorForwardVector` (`self.mSkeleton`))))
  (:`Pressed`
    (if (== 0 (`self.mCurrentSplit`))
      (bind _returnvalue (`|SpawnActorFromClass` "/Game/SPLITCharacters/Bone.Bone_C" (`self.GetTransform` (`self.mSkeleton`)) "AdjustIfPossibleButAlwaysSpawn" "OverrideRootScale" null null))
      (bind _asbone (cast `/Game/SPLITCharacters/Bone` _returnvalue))
      (if (<= _returnvalue_y 0.0)
        (set `/Game/SPLITCharacters/Bone.mTargetPosition` (+ (`self.K2_GetActorLocation` _returnvalue) (0.0 100.0 0.0)) _asbone)
        (else
          (set `/Game/SPLITCharacters/Bone.mTargetPosition` (+ (`self.K2_GetActorLocation` _returnvalue) (0.0 -100.0 0.0)) _asbone))))))

(event `InputAction|Switch`
  (params (Key :type "Key Structure"))
  (bind _returnvalue (`GameplayStatics.GetPlayerController` 0))
  (:`Pressed`
    (`self.UnPossess` _returnvalue)
    (switch `int` (`self.mCurrentSplit`)
      (:`0`
        (set `self.mCurrentSound` (`self.mSkinSound`))
        (`self.Possess` _returnvalue (`self.mSkin`)))
      (:`1`
        (set `self.mCurrentSound` (`self.mMuscleSound`))
        (`self.Possess` _returnvalue (`self.mMuscle`)))
      (:`2`
        (set `self.mCurrentSound` (`self.mSkeletonSound`))
        (`self.Possess` _returnvalue (`self.mSkeleton`))))
    (set `self.mCurrentSplit` (mod (+ (`self.mCurrentSplit`) 1) 3))
    (`ActorComponent.SetActive` (`self.mPlayingSound`) false true)
    (set `self.mPlayingSound` null)))

(event `self.ReceiveTick`
  (params (DeltaSeconds :type "Float (single-precision)"))
  (bind _mplayingsound (`self.mPlayingSound`))
  (`|ExecutionSequence`
    (:`then_0`
      (if (or (`self.IsInputKeyDown` "D") (`self.IsInputKeyDown` "A"))
        (`|ExecutionSequence`
          (:`then_0`
            ;[1 1 1] If the player is walking and no sound is currently being played.
            (`/Engine/EditorBlueprintResources/StandardMacros.IsValid` (`self.mPlayingSound`)
              (:`Is Not Valid`
                ;[1 1 1] Spawn the current Split Walking sound and assign it to the current playing sound.
                (bind _returnvalue (`GameplayStatics.SpawnSound2D` (`self.mCurrentSound`) 1.0 1.0 0.0 null))
                (set `self.mPlayingSound` _returnvalue))))
          (:`then_1`
            (if (`self.IsInputKeyDown` "D")
              (set `self.mForce` (`KismetMathLibrary.MakeVector` 0.0 10000.0))
              (else
                (set `self.mForce` (`KismetMathLibrary.MakeVector` 0.0 -10000.0))))))
        (else
          ;[1 1 1] If the player isn't walking, turn off the walking sound and set it to null.
          (`/Engine/EditorBlueprintResources/StandardMacros.IsValid` _mplayingsound
            (:`Is Valid`
              (`ActorComponent.SetActive` _mplayingsound false true)
              (set `self.mPlayingSound` null))))))
    (:`then_1`
      ;[1 1 1] Apply a constant force on the Player Controller possessed Pawn
      (`PrimitiveComponent.AddForce` (`MovementComponent.UpdatedPrimitive` (`Pawn.GetMovementComponent` (`self.K2_GetPawn` (`GameplayStatics.GetPlayerController` 0)))) (`self.mForce`) "None" false))))

(fn `UserConstructionScript`)